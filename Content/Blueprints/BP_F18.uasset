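; BP_F18 is an F-18 fighter jet pawn that takes player input for camera look and throttle.
; On BeginPlay it adds the IMC_FighterJet Enhanced Input mapping context to the first player controller.
; Look input feeds controller yaw and pitch.
; Thrust and brake both ease a shared ThrottleValue toward their action value with FInterpTo, then pass it to the vehicle movement component's throttle input.
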(event Input|EnhancedActionEvents|EnhancedInputActionIA_LookAround
  (params (ActionValue :type Vector%202D%20Structure) (ElapsedSeconds :type Float%20%28double-precision%29) (TriggeredSeconds :type Float%20%28double-precision%29) (InputAction :type Input%20Action%20Object%20Reference :default "/Game/Inputs/FlightInput/IA_LookAround.IA_LookAround"))
  (bind (_x _y) (Math|Vector2D|BreakVector2D ActionValue))
  (Pawn|Input|AddControllerYawInput _x)
  (Pawn|Input|AddControllerPitchInput _y))

(event Input|EnhancedActionEvents|EnhancedInputActionIA_Thrust
  (params (ActionValue :type Float%20%28double-precision%29) (ElapsedSeconds :type Float%20%28double-precision%29) (TriggeredSeconds :type Float%20%28double-precision%29) (InputAction :type Input%20Action%20Object%20Reference :default "/Game/Inputs/FlightInput/IA_Thrust.IA_Thrust"))
  (bind _output_get (Variables|Default|SetThrottle%20Value (Math|Interpolation|FInterpTo (Variables|Default|GetThrottle%20Value) ActionValue (Utilities|Time|GetWorldDeltaSeconds) 0.5)))
  (Class|ChaosVehicleMovementComponent|SetThrottleInput (Variables|Default|GetVehicleMovementComponent) _output_get))

(event Input|EnhancedActionEvents|EnhancedInputActionIA_Brake
  (params (ActionValue :type Float%20%28double-precision%29) (ElapsedSeconds :type Float%20%28double-precision%29) (TriggeredSeconds :type Float%20%28double-precision%29) (InputAction :type Input%20Action%20Object%20Reference :default "/Game/Inputs/FlightInput/IA_Brake.IA_Brake"))
  (bind _output_get (Variables|Default|SetThrottle%20Value (Math|Interpolation|FInterpTo (Variables|Default|GetThrottle%20Value) ActionValue (Utilities|Time|GetWorldDeltaSeconds) 0.5)))
  (Class|ChaosVehicleMovementComponent|SetThrottleInput (Variables|Default|GetVehicleMovementComponent) _output_get))

(event EventBeginPlay
  (Input|AddMappingContext (PlayerController|LocalPlayerSubsystems|GetEnhancedInputLocalPlayerSubsystem (Game|GetPlayerController 0)) "/Game/Inputs/FighterJet/IMC_FighterJet.IMC_FighterJet" 0 "(bIgnoreAllPressedKeysUntilRelease=True,bForceImmediately=False,bNotifyUserSettings=False)"))

(event Collision|EventActorBeginOverlap
  (params (OtherActor :type Actor%20Object%20Reference)))

(event EventTick
  (params (DeltaSeconds :type Float%20%28single-precision%29)))

(fn ConstructionScript)